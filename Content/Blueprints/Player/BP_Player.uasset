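; BP_Player is the player Blueprint, holding RPG progression, attributes and combat stats.
; BeginPlay adds the WBP_Player widget to the viewport, then sets every stat's default in InitializeVariables.
; Tick watches for Experience changes and levels up only on an exact match with RequiredExperience, resetting experience, scaling the requirement by level and granting attribute points.
; Left mouse press and release fire LMBPressed and LMBReleased calls, with debug prints.
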(event `self.ReceiveBeginPlay`
  (bind _returnvalue (`|CreateWidget` "/Game/UI/WBP_Player.WBP_Player_C"))
  (`UserWidget.AddToViewport` _returnvalue 0)
  (`self.InitializeVariables`))

(event `self.ReceiveTick`
  (params (DeltaSeconds :type "Float (single-precision)"))
  (bind _experience (`self.Experience`))
  (bind _level (`self.Level`))
  (if (not (== _experience (`self.OldExperience`)))
    (set `self.OldExperience` _experience)
    ;[1 1 1] When Required Experience is reached, set the current experience to 0 and add a level
    (if (== (`self.Experience`) (`self.RequiredExperience`))
      (set `self.Experience` 0)
      (set `self.Level` (+ (`self.Level`) 1))
      ;[1 1 1] Increase Required Experience - Formula: (((Level * 5) + Level) + (Level * 2))
      (set `self.RequiredExperience` (+ (+ (* 5 _level) _level) (* _level 2)))
      ;[1 1 1] Add Attribute Points on level up
      (set `self.AttributePoints` (+ (`self.AttributePoints`) 3)))))

(event `Key|LeftMouseButton`
  (params (Key :type "Key Structure"))
  (:`Pressed`
    (`self.LMBPressed`)
    (`KismetSystemLibrary.PrintString` "PressedInBP"))
  (:`Released`
    (`self.LMBReleased`)
    (`KismetSystemLibrary.PrintString` "ReleasedInBP")))

(fn `InitializeVariables`
  ;[1 1 1] Set the values of all Player variables
  (set `self.Level` 0)
  (set `self.Experience` 0)
  (set `self.OldExperience` 0)
  (set `self.AttributePoints` 0)
  (set `self.RequiredExperience` 4)
  (set `self.Strength` 1)
  (set `self.Dexterity` 1)
  (set `self.Intelligence` 1)
  (set `self.Faith` 1)
  (set `self.Endurance` 1)
  (set `self.MaximumLife` 10)
  (set `self.CurrentLife` 10)
  (set `self.Armour` 0)
  (set `self.BlockChance` 0.0)
  (set `self.LifeRegeneration` 0)
  (set `self.PhysicalDamageMinimum` 1)
  (set `self.PhysicalDamageMaximum` 2)
  (set `self.HolyDamageMinimum` 0)
  (set `self.HolyDamageMaximum` 0)
  (set `self.AttacksPerSecond` 2.0)
  (set `self.CriticalStrikeChance` 0.1)
  (set `self.CriticalStrikeMultiplier` 2.0)
  (set `self.ArmourPenetration` 0)
  (set `self.SkillCooldown` 0.0))

(fn `UserConstructionScript`)